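; World object manager that spawns scrolling obstacles and fence posts and moves them along a fixed distance, as in an endless scroller.
; Looping timers add fence posts on both sides and an obstacle in one of three random lanes, each as a child actor component.
; A map tracks each component's start position and progress; while CanMove is set, Tick lerps them forward by Speed and destroys those past the end.
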(event `Create Obsticle`
  (`self.Add Object` "/Game/Blueprints/World/ScrollerObjects/BP_ScrollerOBJ_Obsticle.BP_ScrollerOBJ_Obsticle_C" (`KismetMathLibrary.MakeVector` 0.0 (* (`KismetMathLibrary.RandomIntegerInRange` -1 1) 150.0))))

(event `self.ReceiveBeginPlay`
  (`KismetSystemLibrary.K2_ClearAndInvalidateTimerHandle` (`self.DecoratorTimer`))
  (bind _returnvalue (`KismetSystemLibrary.K2_SetTimerDelegate` (delegate `Add Decorators`) 0.5 true))
  (set `self.DecoratorTimer` _returnvalue)
  (`KismetSystemLibrary.K2_SetTimerDelegate` (delegate `Create Obsticle`) 1.0 true))

(event `Add Decorators`
  (`self.Add Object` "/Game/Blueprints/World/ScrollerObjects/BP_ScrollerOBJ_FencePost.BP_ScrollerOBJ_FencePost_C" (0.0 -300.0 0.0))
  (`self.Add Object` "/Game/Blueprints/World/ScrollerObjects/BP_ScrollerOBJ_FencePost.BP_ScrollerOBJ_FencePost_C" (0.0 300.0 0.0)))

(event `self.ReceiveTick`
  (params (DeltaSeconds :type "Float (single-precision)"))
  (if (`self.CanMove`)
    (`self.Update Objects` DeltaSeconds)))

(fn `Add Object`
  (params (`Object Class` :type "/Game/Blueprints/World/BP_BaseScrollerObject Class Reference") (`Additional Offset` :type "Vector Structure"))
  (bind _returnvalue (+ (`self.SpawnOffset`) `Additional Offset`))
  (bind _returnvalue_2 (`AddComponent|NODE_AddChildActorComponent-0` :`bManualAttachment` true :`RelativeTransform` (`KismetMathLibrary.MakeTransform` _returnvalue (`self.Spawn Offset Rotation`))))
  (`SceneComponent.K2_AttachToComponent` _returnvalue_2 (`self.Object Root`) "None" "KeepWorld" "KeepWorld" "KeepWorld" true)
  (`ChildActorComponent.SetChildActorClass` _returnvalue_2 `Object Class`)
  (`BlueprintMapLibrary.Map_Add` (`self.ObjectTracker`) _returnvalue_2 (make `/Game/Blueprints/Data/Structs/S_ScrollerObjectValue` 0.0 _returnvalue)))

(fn `Update Objects`
  (params (`Delta Time` :type "Float (double-precision)"))
  (locals (FrameAddedScalar :type "Float (double-precision)") (`Child Actors` :type "Array of ChildActorComponent Object Reference") (`Iteration New Scalar` :type "Float (double-precision)"))
  (bind _objecttracker (`self.ObjectTracker`))
  (set `local.FrameAddedScalar` (* `Delta Time` (`self.Speed`)))
  (bind _keys (`BlueprintMapLibrary.Map_Keys` (`self.ObjectTracker`)))
  (bind _output_get (set `local.Child Actors` _keys))
  (for _array_element _output_get
    (bind _output_get_2 (set `local.Iteration New Scalar` (+ (break `/Game/Blueprints/Data/Structs/S_ScrollerObjectValue` (`BlueprintMapLibrary.Map_Find` (`self.ObjectTracker`) _array_element)) (`local.FrameAddedScalar`))))
    (if (> _output_get_2 1.0)
      (`BlueprintMapLibrary.Map_Remove` _objecttracker _array_element)
      (`ActorComponent.K2_DestroyComponent` _array_element)
      (else
        (bind _structout (setmembers `/Game/Blueprints/Data/Structs/S_ScrollerObjectValue` :`StructRef` (`BlueprintMapLibrary.Map_Find` _objecttracker _array_element) :`Scallar` (`local.Iteration New Scalar`)))
        (`BlueprintMapLibrary.Map_Add` (`self.ObjectTracker`) _array_element _structout)
        (bind (_scallar _startingposition) (break `/Game/Blueprints/Data/Structs/S_ScrollerObjectValue` _structout))
        (`SceneComponent.K2_SetWorldLocation` _array_element (`KismetMathLibrary.VLerp` _startingposition (+ _startingposition (`self.LerpMovementDist`)) _scallar) false false)))))

(fn `UserConstructionScript`)