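; BP_PlayerRunner is the player pawn for a lane-based runner, switching between clamped lanes and dying on obstacle contact.
; Enhanced Input left and right actions pass a clamped lane to SetNewLane, which instantly offsets the StaticMesh sideways from its initial position by lane width.
; A Sphere overlap with an actor tagged "Obsticle" triggers Die, which stops BP_WorldObjectManager movement and notifies BP_RunnerPC of the death.
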(event `self.ReceiveBeginPlay`
  (bind _returnvalue (`GameplayStatics.GetActorOfClass` "/Game/Blueprints/World/BP_WorldObjectManager.BP_WorldObjectManager_C"))
  (set `self.WorldObjectManager` _returnvalue)
  (set `self.Initial Offset` (`SceneComponent.RelativeLocation` (`self.StaticMesh`)))
  (bind _asbp_runner_pc (cast `/Game/Blueprints/Core/BP_RunnerPC` (`GameplayStatics.GetPlayerController` 0)))
  (set `self.Runner PC` _asbp_runner_pc))

(event `EnhancedInput|/Game/Blueprints/Input/IA_MoveRight`
  (params (ActionValue :type Boolean) (ElapsedSeconds :type "Float (double-precision)") (TriggeredSeconds :type "Float (double-precision)") (InputAction :type "InputAction Object Reference" :default "/Game/Blueprints/Input/IA_MoveRight.IA_MoveRight"))
  (:`Started`
    (`self.SetNewLane` (`KismetMathLibrary.Clamp` (+ (`self.CurrentLane`) 1) (`self.MinLane`) (`self.MaxLane`)))))

(event `Die`
  (set `/Game/Blueprints/World/BP_WorldObjectManager.CanMove` false (`self.WorldObjectManager`))
  (`/Game/Blueprints/Core/BP_RunnerPC.Player died` (`self.Runner PC`)))

(event `EnhancedInput|/Game/Blueprints/Input/IA_MoveLeft`
  (params (ActionValue :type Boolean) (ElapsedSeconds :type "Float (double-precision)") (TriggeredSeconds :type "Float (double-precision)") (InputAction :type "InputAction Object Reference" :default "/Game/Blueprints/Input/IA_MoveLeft.IA_MoveLeft"))
  (:`Started`
    (`self.SetNewLane` (`KismetMathLibrary.Clamp` (+ (`self.CurrentLane`) -1) (`self.MinLane`) (`self.MaxLane`)))))

(event `self.Sphere.OnComponentBeginOverlap`
  (params (OverlappedComponent :type "PrimitiveComponent Object Reference") (OtherActor :type "Actor Object Reference") (OtherComp :type "PrimitiveComponent Object Reference") (OtherBodyIndex :type Integer) (bFromSweep :type Boolean) (SweepResult :type "HitResult Structure (by ref)"))
  (if (`self.ActorHasTag` OtherActor "Obsticle")
    (`self.Die`)))

(fn `SetNewLane`
  (params (NewLane :type Integer))
  (if (!= NewLane (`self.CurrentLane`))
    (bind _output_get (set `self.CurrentLane` NewLane))
    (`SceneComponent.K2_SetRelativeLocation` (`self.StaticMesh`) (+ (`self.Initial Offset`) (`KismetMathLibrary.MakeVector` 0.0 (* _output_get (`self.LaneWidth`)))) false false)))

(fn `UserConstructionScript`)