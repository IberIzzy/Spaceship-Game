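; BP_RunnerPC is the runner game's player controller, handling input setup and the death and restart flow.
; On BeginPlay it registers the runner Enhanced Input mapping context.
; The Playerdied event shows a death screen widget with the cursor and UI-only input.
; RestartGame hides the cursor, restores game-only input and reopens the runner level.
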(event `Player died`
  (bind _returnvalue (`|CreateWidget` "/Game/Blueprints/UI/WBP_DeathScreen.WBP_DeathScreen_C" self))
  (`UserWidget.AddToViewport` _returnvalue 0)
  (`WidgetBlueprintLibrary.SetInputMode_UIOnlyEx` self _returnvalue)
  (set `self.bShowMouseCursor` true))

(event `Restart Game`
  (set `self.bShowMouseCursor` false)
  (`WidgetBlueprintLibrary.SetInputMode_GameOnly` self)
  (`GameplayStatics.OpenLevel` "RunnerLevel"))

(event `self.ReceiveBeginPlay`
  (`EnhancedInputSubsystemInterface.AddMappingContext` (subsystem `EnhancedInputLocalPlayerSubsystem`) "/Game/Blueprints/Input/IMC_RunnerInput.IMC_RunnerInput" 0 (struct)))

(fn `UserConstructionScript`)